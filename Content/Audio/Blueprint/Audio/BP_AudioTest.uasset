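; BP_AudioTest is an audio test Blueprint that triggers a random ambient one-shot or loop from its set of sound components.
; BesseresOnPlay rolls a random integer and activates one matching component, such as wings, dogs, thunder, bell, crows or voices, with the reset flag varying per sound.
; The event graph and construction script are empty, so nothing in this Blueprint calls the function itself.
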(event EventBeginPlay)

(event Collision|EventActorBeginOverlap
  (params (OtherActor :type Actor%20Object%20Reference)))

(event EventTick
  (params (DeltaSeconds :type Float%20%28single-precision%29)))

(fn ConstructionScript)

(fn BesseresonPlay
  (switch int (Math|Random|RandomIntegerinRange 0 9)
    (:Default
      (Components|Activation|Activate (Variables|Default|GetMS_Male) true))
    (:0
      (Components|Activation|Activate (Variables|Default|GetWings) true))
    (:1
      (Components|Activation|Activate (Variables|Default|GetDogs) true))
    (:2
      (Components|Activation|Activate (Variables|Default|GetMS_Baby) false))
    (:3
      (Components|Activation|Activate (Variables|Default|GetMS_Carriage) false))
    (:4
      (Components|Activation|Activate (Variables|Default|GetMS_Cats) true))
    (:5
      (Components|Activation|Activate (Variables|Default|GetMS_Thunder) false))
    (:6
      (Components|Activation|Activate (Variables|Default|GetMS_Bell) false))
    (:7
      (Components|Activation|Activate (Variables|Default|GetMS_Female) true))
    (:8
      (Components|Activation|Activate (Variables|Default|GetMS_Crows) true))))