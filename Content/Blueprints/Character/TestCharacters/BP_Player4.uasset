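; BP_Player4 is a test fighting-game character with sidestep movement, capsule-resizing duck and pushing of BP_Player2 on contact.
; On BeginPlay it spawns an attached hurtbox actor or collects "CollisionHB" mesh components, then maps Enhanced Input key names to input types.
; Move, duck, attack and throw presses resolve the held key through that map into a time- and frame-stamped input buffer.
; Timelines drive sidestep velocity; buffer pruning exists but is unwired.
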(event OnComponentHit(CapsuleComponent)
  (params (HitComponent :type Primitive%20Component%20Object%20Reference) (OtherActor :type Actor%20Object%20Reference) (OtherComp :type Primitive%20Component%20Object%20Reference) (NormalImpulse :type Vector :default "0, 0, 0") (Hit :type Hit%20Result%20Structure%20%28by%20ref%29))
  (CallFunction|ApplyPushLogic OtherActor 0.8))

(event Input|EnhancedActionEvents|EnhancedInputActionIA_MoveForward
  (params (ActionValue :type Float%20%28double-precision%29) (ElapsedSeconds :type Float%20%28double-precision%29) (TriggeredSeconds :type Float%20%28double-precision%29) (InputAction :type Input%20Action%20Object%20Reference :default "/Game/Blueprints/Pawn/LocalInputActions/IA_MoveForward.IA_MoveForward"))
  (:Started
    (CallFunction|SetInputBufferLogic InputAction)))

(event Input|EnhancedActionEvents|EnhancedInputActionIA_SideStepNegativeY
  (params (ActionValue :type Float%20%28double-precision%29) (ElapsedSeconds :type Float%20%28double-precision%29) (TriggeredSeconds :type Float%20%28double-precision%29) (InputAction :type Input%20Action%20Object%20Reference :default "/Game/Blueprints/Pawn/LocalInputActions/IA_SideStepNegativeY.IA_SideStepNegativeY"))
  ;[1 1 1] OnTap SideStep Movement
  (:Triggered
    (if (Variables|Default|GetIsSideStepNY)
      (Class|FightingCharacter|UpdateCharacterRotation)
      (Timeline|Timeline PlayFromStart
        (:Update
          (Variables|/Script/Engine.MovementComponent|SetVelocity (Variables|Character|GetCharacterMovement) (* (+ (* (Transformation|GetActorRightVector) 0.8 -1.0) (* (Transformation|GetActorForwardVector) 0.2)) (Variables|Default|GetWalkSpeed))))))))

(event Input|EnhancedActionEvents|EnhancedInputActionIA_SideStepPositiveY
  (params (ActionValue :type Float%20%28double-precision%29) (ElapsedSeconds :type Float%20%28double-precision%29) (TriggeredSeconds :type Float%20%28double-precision%29) (InputAction :type Input%20Action%20Object%20Reference :default "/Game/Blueprints/Pawn/LocalInputActions/IA_SideStepPositiveY.IA_SideStepPositiveY"))
  ;[1 1 1] OnTap SideStep Movement
  (:Triggered
    (if (Variables|Default|GetIsSideStepPY)
      (Class|FightingCharacter|UpdateCharacterRotation)
      (Timeline|Timeline_0 PlayFromStart
        (:Update
          (Variables|/Script/Engine.MovementComponent|SetVelocity (Variables|Character|GetCharacterMovement) (* (+ (* (Transformation|GetActorRightVector) 0.8) (* (Transformation|GetActorForwardVector) 0.2)) (Variables|Default|GetWalkSpeed))))))))

(event Input|EnhancedActionEvents|EnhancedInputActionIA_AddToInputBuffer
  (params (ActionValue :type Boolean) (ElapsedSeconds :type Float%20%28double-precision%29) (TriggeredSeconds :type Float%20%28double-precision%29) (InputAction :type Input%20Action%20Object%20Reference :default "/Game/Blueprints/Pawn/LocalInputActions/IA_AddToInputBuffer.IA_AddToInputBuffer")))

(event Input|EnhancedActionEvents|EnhancedInputActionIA_MoveBackward
  (params (ActionValue :type Float%20%28double-precision%29) (ElapsedSeconds :type Float%20%28double-precision%29) (TriggeredSeconds :type Float%20%28double-precision%29) (InputAction :type Input%20Action%20Object%20Reference :default "/Game/Blueprints/Pawn/LocalInputActions/IA_MoveBackward.IA_MoveBackward"))
  (:Started
    (CallFunction|SetInputBufferLogic InputAction)))

(event Input|EnhancedActionEvents|EnhancedInputActionIA_Duck
  (params (ActionValue :type Boolean) (ElapsedSeconds :type Float%20%28double-precision%29) (TriggeredSeconds :type Float%20%28double-precision%29) (InputAction :type Input%20Action%20Object%20Reference :default "/Game/Blueprints/Pawn/LocalInputActions/IA_Duck.IA_Duck"))
  (:Triggered
    (Components|Capsule|SetCapsuleSize (Variables|Default|GetCapsuleComponent) 34.0 44.0 true))
  (:Started
    (CallFunction|SetInputBufferLogic InputAction))
  (:Completed
    (Components|Capsule|SetCapsuleSize (Variables|Default|GetCapsuleComponent) 34.0 88.0 true)))

(event Input|EnhancedActionEvents|EnhancedInputActionIA_LightAttack
  (params (ActionValue :type Boolean) (ElapsedSeconds :type Float%20%28double-precision%29) (TriggeredSeconds :type Float%20%28double-precision%29) (InputAction :type Input%20Action%20Object%20Reference :default "/Game/Blueprints/Pawn/LocalInputActions/IA_LightAttack.IA_LightAttack"))
  (:Started
    (CallFunction|SetInputBufferLogic InputAction)))

(event Input|EnhancedActionEvents|EnhancedInputActionIA_HeavyAttack
  (params (ActionValue :type Boolean) (ElapsedSeconds :type Float%20%28double-precision%29) (TriggeredSeconds :type Float%20%28double-precision%29) (InputAction :type Input%20Action%20Object%20Reference :default "/Game/Blueprints/Pawn/LocalInputActions/IA_HeavyAttack.IA_HeavyAttack"))
  (:Started
    (CallFunction|SetInputBufferLogic InputAction)))

(event Input|EnhancedActionEvents|EnhancedInputActionIA_Throw
  (params (ActionValue :type Boolean) (ElapsedSeconds :type Float%20%28double-precision%29) (TriggeredSeconds :type Float%20%28double-precision%29) (InputAction :type Input%20Action%20Object%20Reference :default "/Game/Blueprints/Pawn/LocalInputActions/IA_Throw.IA_Throw"))
  (:Started
    (CallFunction|SetInputBufferLogic InputAction)))

(event EventBeginPlay
  ;[1 1 1] Spawn Hurtbox and owned by the player
  (CallFunction|SpawnHurtboxes)
  (Utilities|FlowControl|Delay 0.2)
  (CallFunction|SetupInputMappings))

(event EventTick
  (params (DeltaSeconds :type Float%20%28single-precision%29))
  ;[1 1 1] Spawn Hurtbox and owned by the player
)

(fn ConstructionScript)

(fn SpawnHurtboxes
  (bind _self self)
  (if (Variables|Default|GetbUsingComplexHurtboxes)
    (CallFunction|SetComplexHurtboxDetails)
    (else
      (bind _returnvalue (Game|SpawnActorfromClass "/Game/Blueprints/Actor/BP_HurtboxActor.BP_HurtboxActor_C" (Transformation|GetActorTransform (Class|PawnMovementComponent|GetPawnOwner (Variables|Character|GetCharacterMovement))) "Undefined" "MultiplyWithRoot" 0 0))
      (bind _output_get (Variables|Default|SetMainHurtboxRef _returnvalue))
      (Utilities|Array|Add (Variables|Default|GetSimpleHurtboxArray) _output_get)
      (Transformation|AttachActorToActor _output_get _self "None" "SnapToTarget" "SnapToTarget" "SnapToTarget" true)
      (Rendering|SetVisibility (Variables|/Script/Project_Nexus.HitBox|GetHitboxDisplay _returnvalue) true false)
      (Actor|SetOwner _returnvalue _self)
      (for _array_element (Components|GetChildrenComponents (Variables|Character|GetMesh) false)
        (Rendering|SetVisibility _array_element false false)))))

(fn SetComplexHurtboxDetails
  (for _array_element (Components|GetChildrenComponents (Variables|Character|GetMesh) false)
    (bind _asstatic_mesh_component (Utilities|Casting|CastToStaticMeshComponent _array_element))
    (if (Utilities|String|Contains (Utilities|GetObjectName _asstatic_mesh_component) "CollisionHB" true)
      (Utilities|Array|Add (Variables|Default|GetComplexHurtboxArray) _asstatic_mesh_component)))
  (for _array_element_2 (Variables|Default|GetComplexHurtboxArray)
    (Rendering|SetVisibility _array_element_2 true false)))

(fn ModifyHurtbox)

(fn ResetHurtbox)

(fn GetActionPressedKeys
  (params (Action :type Input%20Action%20Object%20Reference))
  (bind _returnvalue (Class|EnhancedInputSubsystemInterface|QueryKeysMappedtoAction(Message) (PlayerController|LocalPlayerSubsystems|GetEnhancedInputLocalPlayerSubsystem (Game|GetPlayerController 0)) Action))
  (for _array_element _returnvalue
    (if (Game|Player|IsInputKeyDown (Game|GetPlayerController 0) _array_element)
      (return _array_element))))

(fn SetupInputMappings
  (bind _returnvalue (Game|GetPlayerController 0))
  (bind _returnvalue_2 (PlayerController|LocalPlayerSubsystems|GetEnhancedInputLocalPlayerSubsystem _returnvalue))
  (for _array_element (Class|EnhancedInputSubsystemInterface|QueryKeysMappedtoAction _returnvalue_2 "/Game/Blueprints/Pawn/LocalInputActions/IA_MoveForward.IA_MoveForward")
    (Class|FightingCharacter|AddtoInputMap (Utilities|String|ToString(Text) (Class|KismetInputLibrary|KeyGetDisplayName _array_element true)) "F_Forward"))
  (for _array_element_2 (Class|EnhancedInputSubsystemInterface|QueryKeysMappedtoAction _returnvalue_2 "/Game/Blueprints/Pawn/LocalInputActions/IA_MoveBackward.IA_MoveBackward")
    (Class|FightingCharacter|AddtoInputMap (Utilities|String|ToString(Text) (Class|KismetInputLibrary|KeyGetDisplayName _array_element_2 true)) "F_Backward"))
  (for _array_element_3 (Class|EnhancedInputSubsystemInterface|QueryKeysMappedtoAction _returnvalue_2 "/Game/Blueprints/Pawn/LocalInputActions/IA_Jump.IA_Jump")
    (Class|FightingCharacter|AddtoInputMap (Utilities|String|ToString(Text) (Class|KismetInputLibrary|KeyGetDisplayName _array_element_3 true)) "F_Jump"))
  (for _array_element_4 (Class|EnhancedInputSubsystemInterface|QueryKeysMappedtoAction _returnvalue_2 "/Game/Blueprints/Pawn/LocalInputActions/IA_Duck.IA_Duck")
    (Class|FightingCharacter|AddtoInputMap (Utilities|String|ToString(Text) (Class|KismetInputLibrary|KeyGetDisplayName _array_element_4 true)) "F_Crouch"))
  (for _array_element_5 (Class|EnhancedInputSubsystemInterface|QueryKeysMappedtoAction _returnvalue_2 "/Game/Blueprints/Pawn/LocalInputActions/IA_Block.IA_Block")
    (Class|FightingCharacter|AddtoInputMap (Utilities|String|ToString(Text) (Class|KismetInputLibrary|KeyGetDisplayName _array_element_5 true)) "F_Block"))
  (for _array_element_6 (Class|EnhancedInputSubsystemInterface|QueryKeysMappedtoAction _returnvalue_2 "/Game/Blueprints/Pawn/LocalInputActions/IA_LightAttack.IA_LightAttack")
    (Class|FightingCharacter|AddtoInputMap (Utilities|String|ToString(Text) (Class|KismetInputLibrary|KeyGetDisplayName _array_element_6 true)) "F_LightAttack"))
  (for _array_element_7 (Class|EnhancedInputSubsystemInterface|QueryKeysMappedtoAction _returnvalue_2 "/Game/Blueprints/Pawn/LocalInputActions/IA_HeavyAttack.IA_HeavyAttack")
    (Class|FightingCharacter|AddtoInputMap (Utilities|String|ToString(Text) (Class|KismetInputLibrary|KeyGetDisplayName _array_element_7 true)) "F_HeavyAttack"))
  (for _array_element_8 (Class|EnhancedInputSubsystemInterface|QueryKeysMappedtoAction _returnvalue_2 "/Game/Blueprints/Pawn/LocalInputActions/IA_Throw.IA_Throw")
    (Class|FightingCharacter|AddtoInputMap (Utilities|String|ToString(Text) (Class|KismetInputLibrary|KeyGetDisplayName _array_element_8 true)) "F_Throw")))

(fn SetupInputAxes)

(fn PerformInputLogic
  (params (Keys :type Key%20Structure :default "None"))
  (Class|FightingCharacter|AddInputtoInputBuffer (Utilities|Struct|MakeInputInfo (.Value (Utilities|Map|Find (Variables|Default|GetInputToInputTypeMap) (Utilities|String|ToString(Text) (Class|KismetInputLibrary|KeyGetDisplayName Keys true)))) "" 0.0 0 false)))

(fn SetInputBufferLogic
  (params (Action :type Input%20Action%20Object%20Reference))
  (bind _array_element (CallFunction|GetActionPressedKeys Action))
  (Class|FightingCharacter|AddInputtoInputBuffer (Utilities|Struct|MakeInputInfo (.Value (Utilities|Map|Find (Variables|Default|GetInputToInputTypeMap) (Utilities|String|ToString(Text) (Class|KismetInputLibrary|KeyGetDisplayName _array_element true)))) (Utilities|String|ToString(Text) (Class|KismetInputLibrary|KeyGetDisplayName _array_element true)) (Utilities|Time|GetTimeSeconds) (Utilities|GetFrameCount) false)))

(fn RemoveOldInputs
  (params (CharacterReference :type Fighting%20Character%20Object%20Reference))
  (bind _indicestoremove (LocalVariables|GetIndicesToRemove))
  (bind _returnvalue (Utilities|Array|LastIndex _indicestoremove))
  (for _index (range 0 (Utilities|Array|LastIndex (Variables|/Script/Project_Nexus.FightingCharacter|GetInputBuffer CharacterReference)))
    (if (< (.TimeStamp (Utilities|Struct|BreakInputInfo (Utilities|Array|Get(acopy) (Variables|/Script/Project_Nexus.FightingCharacter|GetInputBuffer CharacterReference) _index))) (- (Utilities|Time|GetTimeSeconds) 0.3))
      (Utilities|Array|AddUnique (LocalVariables|GetIndicesToRemove) _index)))
  (for _index_2 (range 0 _returnvalue)
    (Utilities|Array|RemoveIndex (Variables|/Script/Project_Nexus.FightingCharacter|GetInputBuffer CharacterReference) (- _returnvalue _index_2)))
  (Utilities|Array|Clear _indicestoremove))

(fn ApplyPushLogic
  (params (InputPin :type Actor%20Object%20Reference) (PushAmount :type Float%20%28double-precision%29))
  (bind _self self)
  (bind _characterstate (Variables|Default|GetCharacterState))
  (bind _returnvalue (Transformation|GetActorForwardVector _self))
  (bind _returnvalue_2 (* _returnvalue PushAmount))
  (if (Math|Boolean|ORBoolean (Utilities|Enum|Equal(Enum) _characterstate "FC_MovingForward") (Utilities|Enum|Equal(Enum) _characterstate "FC_MovingBackward") (Utilities|Enum|Equal(Enum) _characterstate "FC_RunningForward") (Utilities|Enum|Equal(Enum) _characterstate "FC_DashForward") (Utilities|Enum|Equal(Enum) _characterstate "FC_DashBackward"))
    (bind _asbp_player_2 (Utilities|Casting|CastToBP_Player2 InputPin))
    (if (Math|Boolean|ORBoolean (Utilities|Enum|Equal(Enum) (Variables|/Script/Project_Nexus.FightingCharacter|GetCharacterState _asbp_player_2) "FC_Default") (Utilities|Enum|Equal(Enum) (Variables|/Script/Project_Nexus.FightingCharacter|GetCharacterState _asbp_player_2) "FC_Blocking") (Utilities|Enum|Equal(Enum) (Variables|/Script/Project_Nexus.FightingCharacter|GetCharacterState _asbp_player_2) "FC_Crouching") (Utilities|Enum|Equal(Enum) (Variables|/Script/Project_Nexus.FightingCharacter|GetCharacterState _asbp_player_2) "FC_CrouchBlocking"))
      (Transformation|AddActorWorldOffset _asbp_player_2 (Math|Vector|MakeVector (.x _returnvalue_2) (.y _returnvalue_2) 0.0) true))))