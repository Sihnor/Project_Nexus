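; BP_HostActor is a world-space prompt actor for hosting an online lobby with the H key.
; Beginning an overlap shows InteractText, enlarges DisplayText and applies the hover color.
; Ending the overlap hides InteractText, restores DisplayText's size and color, and resets its text to the host prompt.
; The graph handles only this visual feedback, with no key input or session logic.
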(event Collision|EventActorBeginOverlap
  (params (OtherActor :type Actor%20Object%20Reference))
  (bind _displaytext (Variables|Default|GetDisplayText))
  (Rendering|SetVisibility (Variables|Default|GetInteractText) true false)
  (Rendering|Components|TextRender|SetWorldSize _displaytext (+ (Variables|Default|GetTextSize) 1e+01))
  (Rendering|Components|TextRender|SetTextRenderColor _displaytext (Variables|Default|GetHoveredColor)))

(event Collision|EventActorEndOverlap
  (params (OtherActor :type Actor%20Object%20Reference))
  (bind _displaytext (Variables|Default|GetDisplayText))
  (Rendering|SetVisibility (Variables|Default|GetInteractText) false false)
  (Rendering|Components|TextRender|SetWorldSize _displaytext (Variables|Default|GetTextSize))
  (Rendering|Components|TextRender|SetTextRenderColor _displaytext (Variables|Default|GetTextColor))
  (Rendering|Components|TextRender|SetText _displaytext (Utilities|Text|FormatText "PRESS H KEY TO HOST A LOBBY")))

(fn ConstructionScript)