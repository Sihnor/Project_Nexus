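; BP_JoinActor is an in-world prompt actor for joining an online lobby, handling only the visual feedback.
; On overlap begin it reveals InteractText, enlarges and recolors DisplayText, and changes it to "HOSTING..." despite its join role.
; On overlap end it hides InteractText and restores the size and color with the J-key join prompt.
; It checks no overlapping actor type and contains no input or session logic.
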(event Collision|EventActorBeginOverlap
  (params (OtherActor :type Actor%20Object%20Reference))
  (bind _displaytext (Variables|Default|GetDisplayText))
  (Rendering|SetVisibility (Variables|Default|GetInteractText) true false)
  (Rendering|Components|TextRender|SetWorldSize _displaytext (+ (Variables|Default|GetTextSize) 1e+01))
  (Rendering|Components|TextRender|SetTextRenderColor _displaytext (Variables|Default|GetHoveredColor))
  (Rendering|Components|TextRender|SetText (Variables|Default|GetDisplayText) (Utilities|Text|FormatText "HOSTING...")))

(event Collision|EventActorEndOverlap
  (params (OtherActor :type Actor%20Object%20Reference))
  (bind _displaytext (Variables|Default|GetDisplayText))
  (Rendering|SetVisibility (Variables|Default|GetInteractText) false false)
  (Rendering|Components|TextRender|SetWorldSize _displaytext (Variables|Default|GetTextSize))
  (Rendering|Components|TextRender|SetTextRenderColor _displaytext (Variables|Default|GetTextColor))
  (Rendering|Components|TextRender|SetText _displaytext (Utilities|Text|FormatText "PRESS J KEY TO JOIN A LOBBY")))

(fn ConstructionScript)