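; BP_CameraEdge is a camera-edge wall that makes launched fighting characters bounce off it.
; When its Cube is hit and CanBounce is set, a FightingCharacter that WasLaunched but not yet wall-bounced is relaunched and flagged IsWallBounce.
; BounceDistance builds the launch velocity from the opponent's reversed forward vector scaled by pushback, adding the opponent's world location to X and Y, with fixed lift.
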(event OnComponentHit(Cube)
  (params (HitComponent :type Primitive%20Component%20Object%20Reference) (OtherActor :type Actor%20Object%20Reference) (OtherComp :type Primitive%20Component%20Object%20Reference) (NormalImpulse :type Vector :default "0, 0, 0") (Hit :type Hit%20Result%20Structure%20%28by%20ref%29))
  (if (Variables|Default|GetCanBounce)
    (bind _asfighting_character (Utilities|Casting|CastToFightingCharacter OtherActor))
    (if (Variables|/Script/Project_Nexus.FightingCharacter|GetWasLaunched _asfighting_character)
      (if (not (Variables|/Script/Project_Nexus.FightingCharacter|GetIsWallBounce _asfighting_character))
        (bind (_xaxis _yaxis _zaxis) (CallFunction|BounceDistance (Variables|/Script/Project_Nexus.FightingCharacter|GetPushBackAmount _asfighting_character) (Variables|/Script/Project_Nexus.FightingCharacter|GetOtherCharacter _asfighting_character) 2e+02))
        (Character|LaunchCharacter _asfighting_character (Math|Vector|MakeVector _xaxis _yaxis _zaxis) true true)
        (Variables|/Script/Project_Nexus.FightingCharacter|SetIsWallBounce _asfighting_character true)))))

(event EventBeginPlay)

(event Collision|EventActorBeginOverlap
  (params (OtherActor :type Actor%20Object%20Reference)))

(event EventTick
  (params (DeltaSeconds :type Float%20%28single-precision%29)))

(fn ConstructionScript)

(fn BounceDistance
  (params (Distance :type Float%20%28double-precision%29) (Player%20Ref :type Actor%20Object%20Reference) (Distance%20ZAxis :type Float%20%28double-precision%29))
  (bind _returnvalue (Transformation|GetActorForwardVector Player%20Ref))
  (bind _returnvalue_2 (Transformation|GetActorLocation Player%20Ref))
  (bind _returnvalue_3 (* Distance 4.0))
  (return (+ (* (* (.x _returnvalue) -1.0) _returnvalue_3) (.x _returnvalue_2)) (+ (* (* (.y _returnvalue) -1.0) _returnvalue_3) (.y _returnvalue_2)) Distance%20ZAxis))