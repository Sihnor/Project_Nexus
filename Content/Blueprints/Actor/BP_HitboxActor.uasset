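; Fighting-game hitbox actor that shows a box colored by type and tests it against the indexed player's hurtboxes when spawned.
; Collision uses component overlap for complex hurtboxes or actor overlap for simple ones.
; Active hits apply stun and pushback, plus ground bounce and GameState damage unless blocked, while throwboxes flag a landed throw.
; SpawnVFX sphere-traces between boxes to place hit or block Niagara effects, also triggering Wwise sounds and KO VFX.
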(event Custom|SpawnHitbox
  (params (PlayerIndex :type Integer))
  (switch Utilities|FlowControl|Switch|SwitchonEHitBoxStates (Variables|Default|GetHitboxType)
    (:HB_Begin
      (Rendering|Material|SetMaterial (Variables|Default|GetHitboxDisplay) 0 "/Game/Assets/Materials/Hitbox/M_BeginHitbox.M_BeginHitbox"))
    (:HB_Active
      (Rendering|Material|SetMaterial (Variables|Default|GetHitboxDisplay) 0 "/Game/Assets/Materials/Hitbox/M_ActiveHitbox.M_ActiveHitbox"))
    (:HB_Hurtbox
      (Rendering|Material|SetMaterial (Variables|Default|GetHitboxDisplay) 0 "/Game/Assets/Materials/Hitbox/M_Hurtbox.M_Hurtbox"))
    (:HB_Throwbox
      (Rendering|Material|SetMaterial (Variables|Default|GetHitboxDisplay) 0 "/Game/Assets/Materials/Hitbox/M_ThrowHitbox.M_ThrowHitbox")))
  (Transformation|SetWorldLocationAndRotation (Variables|Default|GetHitboxDisplay) (Variables|Default|GetHitboxLocation) (Variables|Default|GetHitboxRotation) false false)
  (Rendering|SetVisibility (Variables|Default|GetHitboxDisplay) (Variables|Default|GetIsHitboxVisible) false)
  (CallFunction|CheckCollision PlayerIndex))

(event Custom|CheckCollision
  (params (PlayerIndex :type Integer))
  (bind _pushbackdistance (Variables|Default|GetPushbackDistance))
  (bind _hitstuntime (Variables|Default|GetHitstunTime))
  (bind _gamemoderef (Variables|Default|GetGameModeRef))
  (bind _asfighting_character (Utilities|Casting|CastToFightingCharacter (Game|GetPlayerCharacter PlayerIndex)))
  (if (Variables|/Script/Project_Nexus.FightingCharacter|GetbUsingComplexHurtboxes _asfighting_character)
    (bind (_bhascollision _hurtbox _hitbox_display) (CallFunction|CheckComplexCollision PlayerIndex))
    (if _bhascollision
      (Utilities|IsValid (Utilities|Array|Get(acopy) (Variables|/Script/Project_Nexus.FightingCharacter|GetComplexHurtboxArray _asfighting_character))
        (:Is%20Valid
          (switch Utilities|FlowControl|Switch|SwitchonEHitBoxStates (Variables|Default|GetHitboxType) :!label _label
            (:HB_Active
              (CallFunction|CheckAlive)
              (Class|FightingCharacter|GetStunned _asfighting_character _hitstuntime (Variables|Default|GetBlockstunTime) _pushbackdistance (Variables|Default|GetLaunchDistance) (Variables|Default|GetIsNeutral) (Variables|Default|GetHitStopTime))
              (CallFunction|SpawnVFX _hitbox_display _hurtbox _hitstuntime false false _asfighting_character)
              (Variables|/Script/Project_Nexus.FightingCharacter|SetPushBackAmount _asfighting_character _pushbackdistance)
              (if (or (and (Utilities|Enum|NotEqual(Enum) (Variables|/Script/Project_Nexus.FightingCharacter|GetCharacterState _asfighting_character) "FC_BlockStunned") (Utilities|Enum|NotEqual(Enum) (Variables|/Script/Project_Nexus.FightingCharacter|GetCharacterState _asfighting_character) "FC_BlockCrouchStunned")) (Variables|/Script/Project_Nexus.FightingCharacter|GetHasLandedThrow _asfighting_character))
                (Variables|/Script/Project_Nexus.FightingCharacter|SetIsGroundBounce _asfighting_character (Variables|Default|GetCauseGroundBounce))
                (Utilities|IsValid _gamemoderef
                  (:Is%20Valid
                    (if (not (Variables|/Game/Blueprints/GameMode/BP_GameModeNexus.BP_GameModeNexus_C|GetIsPlayerDead _gamemoderef))
                      (Class|NexusGameState|RefreshHealth (Variables|Default|GetGameStateRef) (Utilities|Enum|ByteToEnumEPlayerEnum (Math|Conversions|ToByte(Integer) PlayerIndex)) (Variables|Default|GetHitboxDamage)))))
                (else
                  (CallFunction|SpawnVFX _hitbox_display _hurtbox 0.0 false true _asfighting_character))))
            (:HB_Throwbox
              (Variables|/Script/Project_Nexus.FightingCharacter|SetHasLandedThrow _asfighting_character true)
              (CallFunction|SpawnVFX _hitbox_display _hurtbox (Variables|Default|GetHitstunTime) true false _asfighting_character))))))
    (else
      (Utilities|IsValid _asfighting_character
        (:Is%20Valid
          (Utilities|IsValid (Utilities|Array|Get(acopy) (Variables|/Script/Project_Nexus.FightingCharacter|GetSimpleHurtboxArray _asfighting_character))
            (:Is%20Valid
              (if (Collision|IsOverlappingActor (Utilities|Array|Get(acopy) (Variables|/Script/Project_Nexus.FightingCharacter|GetSimpleHurtboxArray _asfighting_character)) :!class /Script/Engine.Actor)
                (goto _label)))))))))

(event Custom|CustomEvent)

(event EventBeginPlay
  (bind _asnexus_game_state (Utilities|Casting|CastToNexus_GameState (Game|GetGameState)))
  (Variables|Default|SetGameStateRef _asnexus_game_state)
  (bind _asbp_game_mode_nexus (Utilities|Casting|CastToBP_GameModeNexus (Game|GetGameMode)))
  (Variables|Default|SetGameModeRef _asbp_game_mode_nexus))

(fn ConstructionScript)

(fn CheckComplexCollision
  (params (PlayerIndex :type Integer))
  (bind _hitboxdisplay (Variables|Default|GetHitboxDisplay))
  (bind _asfighting_character (Utilities|Casting|CastToFightingCharacter (Game|GetPlayerCharacter PlayerIndex)))
  (bind _array_element (Utilities|Array|ForEachLoopwithBreak (Variables|/Script/Project_Nexus.FightingCharacter|GetComplexHurtboxArray _asfighting_character) :!label _label)
    (:LoopBody
      (if (Class|PrimitiveComponent|IsOverlappingComponent _array_element _hitboxdisplay)
        (Variables|Default|SetCollisionOccurred true)
        (goto _label Break)))
    (:Completed
      (return (Variables|Default|GetCollisionOccurred) _array_element _hitboxdisplay))))

(fn SpawnVFX
  (params (Hitbox :type Static%20Mesh%20Component%20Object%20Reference) (Hurtbox :type Static%20Mesh%20Component%20Object%20Reference) (HitStunTime :type Float%20%28double-precision%29) (IsThrow :type Boolean) (GotBlocked :type Boolean) (FC%20Ref :type Fighting%20Character%20Object%20Reference))
  (bind _returnvalue (Transformation|GetWorldLocation Hitbox))
  (bind _returnvalue_2 (Transformation|GetWorldLocation Hurtbox))
  (bind _returnvalue_3 (* HitStunTime 2.0))
  (bind _playerindex (Variables|/Script/Project_Nexus.FightingCharacter|GetPlayerIndex FC%20Ref))
  (bind _haslandedthrow (Variables|/Script/Project_Nexus.FightingCharacter|GetHasLandedThrow FC%20Ref))
  (bind _returnvalue_4 (not _haslandedthrow))
  (bind _returnvalue_5 (* _returnvalue_3 2.0))
  (bind _outhit (Collision|SphereTraceByChannel _returnvalue_2 (Math|Vector|MakeVector (.x _returnvalue) (.y _returnvalue) (.Z (Math|Vector|BreakVector _returnvalue_2))) 25.0 "TraceTypeQuery1" false 0 "None"))
  (if IsThrow
    (bind (_xaxis _yaxis _zaxis) (CallFunction|DistanceLogic -2e+01 FC%20Ref 5e+01))
    (Niagara|SpawnSystematLocation "/Game/Assets/VFX/ParticleSystems/NS_VFXGrabbed.NS_VFXGrabbed" (Math|Vector|MakeVector _xaxis _yaxis _zaxis))
    (elif GotBlocked
      (Niagara|SpawnSystematLocation "/Game/Assets/VFX/ParticleSystems/NS_VFXBlock.NS_VFXBlock" (.location _outhit))
      (elif (> HitStunTime 0.5)
        (Niagara|SpawnSystematLocation "/Game/Assets/VFX/ParticleSystems/NS_VFXHeavyHit.NS_VFXHeavyHit" (.location _outhit))
        (if _returnvalue_4
          (if (== _playerindex 0)
            (Class|AkGameplayStatics|PostEvent "/Game/WwiseAudio/Events/Player/PlayerCombat/Play_Player_Punch_Heavy.Play_Player_Punch_Heavy")
            (bind _asbp_player_2 (Utilities|Casting|CastToBP_Player2 FC%20Ref))
            (Default|SpawnKOVFX _asbp_player_2 _returnvalue_3 "StunDuration")
            (else
              (Class|AkGameplayStatics|PostEvent "/Game/WwiseAudio/Events/Player2/Player2Combat/Play_Player2_Punch_Heavy.Play_Player2_Punch_Heavy")
              (bind _asbp_player_1 (Utilities|Casting|CastToBP_Player1 FC%20Ref))
              (Default|SpawnKOVFX _asbp_player_1 _returnvalue_3 "StunDuration"))))
        (else
          (Niagara|SpawnSystematLocation "/Game/Assets/VFX/ParticleSystems/NS_VFXLightHit.NS_VFXLightHit" (.location _outhit))
          (if _returnvalue_4
            (if (== _playerindex 0)
              (Class|AkGameplayStatics|PostEvent "/Game/WwiseAudio/Events/Player/PlayerCombat/Play_Player_Punch_Light.Play_Player_Punch_Light")
              (bind _asbp_player_2_2 (Utilities|Casting|CastToBP_Player2 FC%20Ref))
              (Default|SpawnKOVFX _asbp_player_2_2 _returnvalue_5 "StunDuration")
              (else
                (Class|AkGameplayStatics|PostEvent "/Game/WwiseAudio/Events/Player2/Player2Combat/Play_Player2_Punch_Light.Play_Player2_Punch_Light")
                (bind _asbp_player_1_2 (Utilities|Casting|CastToBP_Player1 FC%20Ref))
                (Default|SpawnKOVFX _asbp_player_1_2 _returnvalue_5 "StunDuration")))))))))

(fn DistanceLogic
  (params (Distance :type Float%20%28double-precision%29) (Player%20Ref :type Actor%20Object%20Reference) (Distance%20ZAxis :type Float%20%28double-precision%29))
  (bind _returnvalue (Transformation|GetActorForwardVector Player%20Ref))
  (bind _returnvalue_2 (Transformation|GetActorLocation Player%20Ref))
  (return (+ (* (.x _returnvalue) Distance) (.x _returnvalue_2)) (+ (* (.y _returnvalue) Distance) (.y _returnvalue_2)) (+ Distance%20ZAxis (.z _returnvalue_2))))

(fn CheckAlive
  (bind _gamemoderef (Variables|Default|GetGameModeRef))
  (Utilities|IsValid _gamemoderef
    (:Is%20Valid
      (if (not (Variables|/Game/Blueprints/GameMode/BP_GameModeNexus.BP_GameModeNexus_C|GetIsPlayerDead _gamemoderef))
        _))))