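; BP_CameraFocusActor is a shared camera rig that frames the two local players, BP_Player1 and BP_Player2.
; Each Tick it moves to their XY midpoint, with height from one-eighth of their summed Z, floored at the first valid frame's value.
; It yaws along the line between them and sets spring arm length to half their distance, clamped.
; BP_CameraEdge boundary spawning and placement exist but are disconnected.
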(event EventBeginPlay)

(event EventTick
  (params (DeltaSeconds :type Float%20%28single-precision%29))
  (bind _asbp_player_1 (Utilities|Casting|CastToBP_Player1 (Game|Player|GetPlayerPawn 0)))
  (bind _asbp_player_2 (Utilities|Casting|CastToBP_Player2 (Game|Player|GetPlayerPawn 1)))
  (if (and (Utilities|IsValid _asbp_player_2) (Utilities|IsValid _asbp_player_1))
    (if (Variables|Default|GetHasSetCameraBounds)
      _
      (else
        (Variables|Default|SetCameraHeightMinimum (/ (+ (.Z (Math|Vector|BreakVector (Transformation|GetActorLocation _asbp_player_2))) (.Z (Math|Vector|BreakVector (Transformation|GetActorLocation _asbp_player_1)))) 8.0))
        (Variables|Default|SetHasSetCameraBounds true)))
    (Transformation|SetActorLocation (Math|Vector|MakeVector (/ (+ (.X (Math|Vector|BreakVector (Transformation|GetActorLocation _asbp_player_2))) (.X (Math|Vector|BreakVector (Transformation|GetActorLocation _asbp_player_1)))) 2.0) (/ (+ (.Y (Math|Vector|BreakVector (Transformation|GetActorLocation _asbp_player_2))) (.Y (Math|Vector|BreakVector (Transformation|GetActorLocation _asbp_player_1)))) 2.0) (Math|Float|Clamp(Float) (/ (+ (.Z (Math|Vector|BreakVector (Transformation|GetActorLocation _asbp_player_2))) (.Z (Math|Vector|BreakVector (Transformation|GetActorLocation _asbp_player_1)))) 8.0) (Variables|Default|GetCameraHeightMinimum) 1e+05)) false false)
    (Transformation|SetActorRotation (Math|Rotator|MakeRotator 0.0 0.0 (.yaw (Math|Rotator|FindLookatRotation (Transformation|GetActorLocation _asbp_player_1) (Transformation|GetActorLocation _asbp_player_2)))))
    (Variables|/Script/Engine.SpringArmComponent|SetTargetArmLength (Variables|Default|GetSpringArmComp) (Math|Float|Clamp(Float) (/ (Math|Float|Absolute(Float) (Math|Vector|Distance(Vector) (Transformation|GetActorLocation _asbp_player_2) (Transformation|GetActorLocation _asbp_player_1))) 2.0) 2.5e+02 4.5e+02))))

(fn ConstructionScript)

(fn CalcuateDistanceOfAxes
  (params (A :type Float%20%28double-precision%29) (B :type Float%20%28double-precision%29))
  (return (+ (/ (- A B) 2.0) B)))

(fn SetCameraBondaries
  (params (Player1 :type BP%20Player%201%20Object%20Reference) (Player2 :type %20Object%20Reference))
  (bind _returnvalue (Game|Player|GetPlayerPawn 1))
  (bind _returnvalue_2 (Game|Player|GetPlayerPawn 0))
  (bind _returnvalue_3 (Transformation|GetActorLocation _returnvalue))
  (bind _returnvalue_4 (Transformation|GetActorLocation _returnvalue_2))
  (bind (_x _y _z) (Math|Vector|BreakVector _returnvalue_3))
  (bind (_x_2 _y_2 _z_2) (Math|Vector|BreakVector _returnvalue_4))
  (Utilities|IsValid _returnvalue_2
    (:Is%20Valid
      (Utilities|IsValid _returnvalue
        (:Is%20Valid
          (Transformation|SetActorLocation (Variables|Default|GetLeftCameraEdge) (Math|Vector|MakeVector (- _x_2 5e+02) _y_2 _z_2) false false)
          (Transformation|SetActorLocation (Variables|Default|GetRightCameraEdge) (Math|Vector|MakeVector (+ _x 5e+02) _y _z) false false))))))