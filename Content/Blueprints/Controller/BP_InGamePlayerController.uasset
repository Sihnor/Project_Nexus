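; BP_InGamePlayerController is the player controller used during gameplay, handling the pause key and the in-game overlay.
; Pressing Escape casts the game state to GS_IngameState and calls its PauseGame.
; SetOverlay creates a UI_IngameBase widget, stores it, adds it to the viewport and switches input to game-only mode.
; BeginPlay is empty and nothing in this Blueprint calls SetOverlay.
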(event EventBeginPlay)

(event Input|KeyboardEvents|Escape
  (params (Key :type Key%20Structure :default "None"))
  (bind _returnvalue (Game|GetGameState))
  (:Pressed
    (if (Utilities|IsValid _returnvalue)
      (bind _asgs_ingame_state (Utilities|Casting|CastToGS_IngameState _returnvalue))
      (Default|PauseGame _asgs_ingame_state))))

(fn ConstructionScript)

(fn SetOverlay
  (bind _returnvalue (UserInterface|CreateWidget "/Game/UI/UI_IngameBase.UI_IngameBase_C" self))
  (bind _output_get (Variables|Default|SetWidget%20Canvas _returnvalue))
  (UserInterface|Viewport|AddtoViewport _output_get 0)
  (Input|SetInputModeGameOnly self false))